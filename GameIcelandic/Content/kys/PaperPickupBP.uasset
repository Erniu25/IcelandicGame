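; PaperPickupBP is a readable paper note that the player toggles open and closed with Interact while standing in its trigger box.
; Box overlaps with BP_ThirdPersonCharacter set the proximity flag and show or remove a KYSNI widget.
; Picking up plays a sound, displays the widget from the Class variable and hides the mesh.
; Putting down reverses this, and also runs automatically when the character leaves while reading.
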(event `/Game/kys/EvenMoreKMS.Interact`
  (if (`self.IsCloseEnough?`)
    (`self.Toggle Pickup`)))

(event `Toggle Pickup`
  (if (`self.isReading?`)
    (`self.PutDownNote`)
    (else
      (`self.PickupNote`))))

(event `PickupNote`
  (`GameplayStatics.PlaySoundAtLocation` "/Game/audio/PickUpPaper.PickUpPaper" (`SceneComponent.K2_GetComponentLocation` (`self.StaticMesh`)) (struct) 1.0 1.0 0.0 null null null null)
  (bind _returnvalue (`|CreateWidget` (`self.Class`)))
  (`UserWidget.AddToViewport` _returnvalue 0)
  (`SceneComponent.SetVisibility` (`self.StaticMesh`) false false)
  (set `self.isReading?` true))

(event `PutDownNote`
  (`GameplayStatics.PlaySoundAtLocation` "/Game/audio/PutDownPaper.PutDownPaper" (`SceneComponent.K2_GetComponentLocation` (`self.StaticMesh`)) (struct) 1.0 1.0 0.0 null null null null)
  (`Widget.RemoveFromParent` (stale `PickupNote` _returnvalue))
  (`SceneComponent.SetVisibility` (`self.StaticMesh`) true false)
  (set `self.isReading?` false))

(event `self.Box.OnComponentBeginOverlap`
  (params (OverlappedComponent :type "PrimitiveComponent Object Reference") (OtherActor :type "Actor Object Reference") (OtherComp :type "PrimitiveComponent Object Reference") (OtherBodyIndex :type Integer) (bFromSweep :type Boolean) (SweepResult :type "HitResult Structure (by ref)"))
  (cast `/Game/ThirdPerson/Blueprints/BP_ThirdPersonCharacter` OtherActor)
  (set `self.IsCloseEnough?` true)
  (bind _returnvalue (`|CreateWidget` "/Game/kys/KYSNI.KYSNI_C"))
  (`UserWidget.AddToViewport` _returnvalue 0))

(event `self.Box.OnComponentEndOverlap`
  (params (OverlappedComponent :type "PrimitiveComponent Object Reference") (OtherActor :type "Actor Object Reference") (OtherComp :type "PrimitiveComponent Object Reference") (OtherBodyIndex :type Integer))
  (cast `/Game/ThirdPerson/Blueprints/BP_ThirdPersonCharacter` OtherActor)
  (`|ExecutionSequence`
    (:`then_0`
      (set `self.IsCloseEnough?` false)
      (`Widget.RemoveFromParent` (stale `self.Box.OnComponentBeginOverlap` _returnvalue))
      (if (`self.isReading?`)
        (`self.PutDownNote`)))))

(fn `UserConstructionScript`)