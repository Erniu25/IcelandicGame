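; BP_NPC_Child1 is a child NPC Blueprint that shows an interact prompt and moves the game to another level.
; When the third-person character enters TriggerZone, it adds the E_interact widget to the viewport.
; When the character leaves, it removes that widget, plays the WB_Fade animation and, after a short delay, opens MainMapButSequence.
; The level change fires on leaving the zone without any input check, and Dialogue is unused.
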(event `self.TriggerZone.OnComponentBeginOverlap`
  (params (OverlappedComponent :type "PrimitiveComponent Object Reference") (OtherActor :type "Actor Object Reference") (OtherComp :type "PrimitiveComponent Object Reference") (OtherBodyIndex :type Integer) (bFromSweep :type Boolean) (SweepResult :type "HitResult Structure (by ref)"))
  (cast `/Game/ThirdPerson/Blueprints/BP_ThirdPersonCharacter` OtherActor)
  (bind _returnvalue (`|CreateWidget` "/Game/UI/E_interact.E_interact_C"))
  (`UserWidget.AddToViewport` _returnvalue 0))

(event `self.TriggerZone.OnComponentEndOverlap`
  (params (OverlappedComponent :type "PrimitiveComponent Object Reference") (OtherActor :type "Actor Object Reference") (OtherComp :type "PrimitiveComponent Object Reference") (OtherBodyIndex :type Integer))
  (cast `/Game/ThirdPerson/Blueprints/BP_ThirdPersonCharacter` OtherActor)
  (`Widget.RemoveFromParent` (stale `self.TriggerZone.OnComponentBeginOverlap` _returnvalue))
  (bind _returnvalue (`|CreateWidget` "/Game/TeleportToEgill/WB_Fade.WB_Fade_C"))
  (`UserWidget.AddToViewport` _returnvalue 0)
  (`/Game/TeleportToEgill/WB_Fade.FadeAnim` _returnvalue)
  (`KismetSystemLibrary.Delay` 0.5)
  (`GameplayStatics.OpenLevel` "MainMapButSequence"))

(fn `UserConstructionScript`
  (`parent.UserConstructionScript`))