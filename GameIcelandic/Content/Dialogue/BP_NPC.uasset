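; BP_NPC is a dialogue NPC whose trigger zone also drives a death animation and a level change.
; When the third-person character enters, it shows the E_interact prompt and plays a dying animation once.
; On exit, it removes the prompt, plays the WB_Fade animation and opens EgillInHisRoom after a short delay.
; Talk advances an index through the Dialogue array, showing each line in a lazily created, reused WB_Dialogue widget.
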(event `self.TriggerZone.OnComponentBeginOverlap`
  (params (OverlappedComponent :type "PrimitiveComponent Object Reference") (OtherActor :type "Actor Object Reference") (OtherComp :type "PrimitiveComponent Object Reference") (OtherBodyIndex :type Integer) (bFromSweep :type Boolean) (SweepResult :type "HitResult Structure (by ref)"))
  (cast `/Game/ThirdPerson/Blueprints/BP_ThirdPersonCharacter` OtherActor)
  (bind _returnvalue (`|CreateWidget` "/Game/UI/E_interact.E_interact_C"))
  (`UserWidget.AddToViewport` _returnvalue 0)
  (`SkeletalMeshComponent.PlayAnimation` (`self.Mesh`) "/Game/Son2/Dying_Anim_mixamo_com.Dying_Anim_mixamo_com" false)
  (`KismetSystemLibrary.Delay` 4.0))

(event `self.TriggerZone.OnComponentEndOverlap`
  (params (OverlappedComponent :type "PrimitiveComponent Object Reference") (OtherActor :type "Actor Object Reference") (OtherComp :type "PrimitiveComponent Object Reference") (OtherBodyIndex :type Integer))
  (cast `/Game/ThirdPerson/Blueprints/BP_ThirdPersonCharacter` OtherActor)
  (`Widget.RemoveFromParent` (stale `self.TriggerZone.OnComponentBeginOverlap` _returnvalue))
  (bind _returnvalue (`|CreateWidget` "/Game/TeleportToEgill/WB_Fade.WB_Fade_C"))
  (`UserWidget.AddToViewport` _returnvalue 0)
  (`/Game/TeleportToEgill/WB_Fade.FadeAnim` _returnvalue)
  (`KismetSystemLibrary.Delay` 0.5)
  (`GameplayStatics.OpenLevel` "EgillInHisRoom"))

(event `/Game/Dialogue/BPI_Dialogue.Talk`
  (`/Engine/EditorBlueprintResources/StandardMacros.IncrementInt` (`self.TalkIndex`)
    (:`  `
      (if (<= (`self.TalkIndex`) (`KismetArrayLibrary.Array_Length` (`self.Dialogue`)))
        (`self.UI`
          (:`then`
            _)
          (:`else`
            (bind _returnvalue (`|CreateWidget` "/Game/UI/WB_Dialogue.WB_Dialogue_C" (`GameplayStatics.GetPlayerController` 0)))
            (bind _output_get (set `self.UI` _returnvalue))
            (`UserWidget.AddToViewport` _output_get 0)))
        (`TextBlock.SetText` (`/Game/UI/WB_Dialogue.TalkText` (`self.UI`)) (`KismetTextLibrary.Conv_StringToText` (`|GetArrayItem` (`self.Dialogue`) (`self.TalkIndex`))))))))

(fn `UserConstructionScript`)